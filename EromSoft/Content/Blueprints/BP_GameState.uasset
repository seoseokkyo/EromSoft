(event EventBeginPlay
  (bind _astarnished_character (Utilities|Casting|CastToTarnishedCharacter (Game|GetPlayerCharacter 0)))
  (Variables|Default|SetPlayer _astarnished_character))

(event EventTick
  (params (DeltaSeconds :type Float%20%28single-precision%29))
  (if (Variables|/Script/EromSoft.EromSoftCharacter|GetbIsNeedToSpawn (Variables|Default|GetPlayer))
    (if (not (Variables|Default|GetDeadProccessing))
      (Variables|Default|SetDeadProccessing true)
      (bind _returnvalue (UserInterface|CreateWidget "/Game/UI_Eldenring/UI_YouDied.UI_YouDied_C" (Game|GetPlayerController 0)))
      (bind _output_get (Variables|Default|SetDieMessage _returnvalue))
      (UserInterface|Viewport|AddtoViewport _output_get 0)
      (Pawn|UnPossess (Game|GetPlayerController 0))
      (Physics|SetSimulatePhysics (Variables|/Script/Engine.Character|GetMesh (Variables|Default|GetPlayer)) false)
      (bind _newtrack_1 (Timeline|Timeline PlayFromStart)
        (:Update
          (Widget|SetRenderOpacity (Variables|Default|GetDieMessage) _newtrack_1))
        (:Finished
          (Widget|RemovefromParent (Variables|Default|GetDieMessage))
          (bind _asbp_third_person_character (Utilities|Casting|CastToBP_ThirdPersonCharacter (Variables|Default|GetPlayer)))
          (Default|UnLinkUI _asbp_third_person_character)
          (Actor|DestroyActor (Variables|Default|GetPlayer))
          (bind _returnvalue_2 (Game|SpawnActorfromClass "/Game/ThirdPerson/Blueprints/BP_ThirdPersonCharacter.BP_ThirdPersonCharacter_C" (Math|Transform|MakeTransform "0.000000,0.000000,90.000000") "AlwaysSpawn" "MultiplyWithRoot" 0 0))
          (bind _output_get_2 (Variables|Default|SetPlayer _returnvalue_2))
          (Variables|/Script/EromSoft.EromSoftCharacter|SetbIsNeedToSpawn _output_get_2 false)
          (Pawn|Possess (Game|GetPlayerController 0) _output_get_2)
          (bind _asbp_third_person_character_2 (Utilities|Casting|CastToBP_ThirdPersonCharacter (Variables|Default|GetPlayer)))
          (Default|LinkUI _asbp_third_person_character_2)
          (Variables|Default|SetDeadProccessing false))))))

(fn ConstructionScript)