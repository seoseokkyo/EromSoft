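; BP_CollisionComponent is an actor component that detects hits along a socketed mesh, reporting them to the base weapon through OnHit.
; While collision is enabled, Tick runs a multi-sphere object trace between the mesh's start and end sockets, skipping ignored actors.
; Each actor is reported once per activation, because enabling collision clears the already-hit list.
; Functions set the traced mesh, manage ignored actors and expose hit state.
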(event Custom|EnableCollision
  ;[1 1 1] EnableCollision
  (CallFunction|ClearHitActors) ; 시작할 때 이미 맞은애 초기화
  (Variables|Default|SetbIsCollisionEnabled? true))

(event Custom|DisableCollision
  ;[1 1 1] DisableCollision
  (Variables|Default|SetbIsCollisionEnabled? false))

(event Custom|CollisionTrace
  (bind _collisionmeshcomponent (Variables|Default|GetCollisionMeshComponent))
  ;[1 1 1] CollisionTrace로 set hit.
  (bind _outhits (Collision|MultiSphereTraceForObjects (Transformation|GetSocketLocation _collisionmeshcomponent (Variables|Initialization|GetStart%20Socket%20Name)) (Transformation|GetSocketLocation _collisionmeshcomponent (Variables|Initialization|GetEnd%20Socket%20Name)) (Variables|Initialization|GetTrace%20Radius) (Variables|Initialization|GetCollision%20Object%20Types) false (Variables|Default|GetActors%20to%20Ignore) (Variables|Initialization|GetDraw%20Debug%20Type)))
  (for _array_element _outhits
    (bind _output_get (Variables|Default|SetLastHit _array_element))
    ;;[1 1 1] 이미 맞은애가 아니면 넘어가라
    (if (not (Utilities|Array|ContainsItem (Variables|Default|GetAlrreadyHitActors) (.HitActor (Collision|BreakHitResult _output_get))))
      (bind _output_get_2 (Variables|Default|SetHit%20Actor (.HitActor (Collision|BreakHitResult _output_get))))
      (Utilities|Array|Add (Variables|Default|GetAlrreadyHitActors) _output_get_2)
      (Default|CallOnHit (Variables|Default|GetLastHit)) ; 받는 애는 베이스 웨폰
    )))

(event Custom|ClearHitActors
  ;[1 1 1] Call Hit Actor
  (Utilities|Array|Clear (Variables|Default|GetAlrreadyHitActors)))

(event Custom|SetCollisionMesh
  (params (MeshComponent :type Primitive%20Component%20Object%20Reference))
  ;[1 1 1] SetCollisionMeshComponent
  (Variables|Default|SetCollisionMeshComponent MeshComponent))

(event EventBeginPlay)

(event EventTick
  (params (DeltaSeconds :type Float%20%28single-precision%29))
  (if (Variables|Default|GetbIsCollisionEnabled?)
    (CallFunction|CollisionTrace)))

(fn GetAlreadyHitActors
  (return (Variables|Default|GetAlrreadyHitActors)))

(fn IsCollisionEnabled?
  (return (Variables|Default|GetbIsCollisionEnabled?)))

(fn GetLastHit
  (return (Variables|Default|GetLastHit)))

(fn GetColisionMeshComponent
  (return (Variables|Default|GetCollisionMeshComponent)))

(fn AddActortoIgnore
  (params (InActor :type Actor%20Object%20Reference%20%28by%20ref%29))
  (Utilities|Array|AddUnique (Variables|Default|GetActors%20to%20Ignore) InActor))

(fn RemoveAvtortoIgnore
  (params (InActorToRemove :type Actor%20Object%20Reference%20%28by%20ref%29))
  (Utilities|Array|RemoveItem (Variables|Default|GetActors%20to%20Ignore) InActorToRemove))

(fn GetActorstoIgnore
  (return (Variables|Default|GetActors%20to%20Ignore)))