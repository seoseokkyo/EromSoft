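; Base weapon actor for the combat system that sets itself up on its owning character when equipped.
; OnEquipped attaches the weapon to the hand socket if the owner's CombatComponent has combat enabled, otherwise to its attach socket.
; It then registers itself as that component's main weapon and sends its combat type to the character mesh's AnimInstance through a message call.
; The event graph holds only disabled default events.
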(event EventBeginPlay
  (|CallParentFunction) ; 지금 이 노드는 비활성 상태입니다. \n핀을 끌어서 다른 노드를 연결하면 활성화됩니다.
)

(event Collision|EventActorBeginOverlap
  (params (OtherActor :type Actor%20Object%20Reference))
  (|CallParentFunction OtherActor) ; 지금 이 노드는 비활성 상태입니다. \n핀을 끌어서 다른 노드를 연결하면 활성화됩니다.
)

(event EventTick
  (params (DeltaSeconds :type Float%20%28single-precision%29))
  (|CallParentFunction DeltaSeconds) ; 지금 이 노드는 비활성 상태입니다. \n핀을 끌어서 다른 노드를 연결하면 활성화됩니다.
)

(fn ConstructionScript
  (|CallParentFunction))

(fn OnEquipped
  (Variables|Default|SetCombatCombatComponent (Actor|GetComponentbyClass (Components|GetOwner) "/Game/CombatSyetem/Blueprints/Components/CombatComponent.CombatComponent_C"))
  (CallFunction|AttachActor (select (Default|IsCombatEnabled? (Variables|Default|GetCombatCombatComponent)) (Variables|초기화|GetHandSocketName) (Variables|Default|GetAttachSocket%20Name)))
  (Default|SetMainWeapon (Variables|Default|GetCombatCombatComponent) self)
  (Class|AnimInstanceBPI|UpdateCombatType(Message) (Components|SkeletalMesh|GetAnimInstance (Variables|/Script/Engine.Character|GetMesh (.AsCharacter (Utilities|Casting|CastToCharacter (Components|GetOwner))))) (Variables|초기화|GetCombatType)))